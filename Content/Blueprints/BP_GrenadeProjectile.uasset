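; Grenade projectile actor that explodes on a fixed short timer after spawning.
; On BeginPlay it waits, calls Explode, then sets a brief life span to remove itself.
; Explode spawns an explosion particle effect and applies radial damage credited to the instigator, with a debug sphere showing the damage radius.
; Overlap and Tick events are unused, so contact does not trigger detonation.
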(event Custom|Explode
  (bind _returnvalue (Transformation|GetActorLocation))
  (Effects|SpawnEmitteratLocation "/Game/FPS_Weapon_Bundle/WeaponEffects/Explosion/P_Explosion.P_Explosion" _returnvalue)
  (Game|Damage|ApplyRadialDamage 1e+02 _returnvalue (Variables|Default|GetdamageRadius) "/Script/Engine.DamageType" 0 self (Game|GetInstigatorController) false "ECC_Visibility")
  (Rendering|Debug|DrawDebugSphere _returnvalue (Variables|Default|GetdamageRadius) 12 "(R=0.760000,G=0.000000,B=0.000000,A=1.000000)" 2.0 1.0))

(event EventBeginPlay
  (Utilities|FlowControl|Delay 1.0)
  (CallFunction|Explode)
  (Actor|SetLifeSpan 0.5))

(event Collision|EventActorBeginOverlap
  (params (OtherActor :type Actor%20Object%20Reference)))

(event EventTick
  (params (DeltaSeconds :type Float%20%28single-precision%29)))

(fn ConstructionScript)