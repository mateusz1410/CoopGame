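; Test game mode that spawns AI bots and keeps score on kills.
; SpawnNewBot runs an EQS spawn-location query, marks each returned point with a debug sphere and randomly spawns BP_AdvanceAI or the more likely BP_TrackerBot there.
; An actor-killed handler bound on BeginPlay adjusts the killer's SPlayerState score, deducting for player-controlled victims and rewarding other pawn kills, then prints it.
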(event Custom|OnActorKilled_Event
  (params (VictimActor :type Actor%20Object%20Reference) (KillerActor :type Actor%20Object%20Reference) (KillerController :type Controller%20Object%20Reference))
  (bind _returnvalue (Pawn|GetControlledPawn KillerController))
  (Utilities|IsValid KillerController
    (:Is%20Valid
      (Utilities|IsValid VictimActor
        (:Is%20Valid
          (bind _aspawn (Utilities|Casting|CastToPawn VictimActor))
          (if (Pawn|IsPlayerControlled _aspawn)
            (bind _assplayer_state (Utilities|Casting|CastToSPlayerState (Variables|/Script/Engine.Pawn|GetPlayerState _returnvalue)))
            (Class|SPlayerState|AddScore _assplayer_state -5e+01)
            (Development|PrintString (Utilities|String|ToString(Float) (Variables|/Script/Engine.PlayerState|GetScore _assplayer_state)) true true "(R=0.380000,G=0.000000,B=0.000000,A=1.000000)" 5.0)
            (else
              (Utilities|IsValid _returnvalue
                (:Is%20Valid
                  (bind _assplayer_state_2 (Utilities|Casting|CastToSPlayerState (Variables|/Script/Engine.Pawn|GetPlayerState _returnvalue)))
                  (Class|SPlayerState|AddScore _assplayer_state_2 2e+01)
                  (Development|PrintString (Utilities|String|ToString(Float) (Variables|/Script/Engine.PlayerState|GetScore _assplayer_state_2)) true true "(R=0.380000,G=0.000000,B=0.000000,A=1.000000)" 5.0))))))))))

(event Custom|OnQueryFinishedEvent_Event
  (params (QueryInstance :type Env%20Query%20Instance%20Blueprint%20Wrapper%20Object%20Reference) (QueryStatus :type EEnvQueryStatus%20Enum :default "Processing"))
  (bind _resultlocations (AI|EQS|GetQueryResultsasLocations QueryInstance))
  (switch Utilities|FlowControl|Switch|SwitchonEEnvQueryStatus QueryStatus
    (:Success
      (for _array_element _resultlocations
        (Rendering|Debug|DrawDebugSphere _array_element 5e+01 12 "(R=1.000000,G=0.586625,B=0.000000,A=1.000000)" 2.0 2.0)
        (Game|SpawnActorfromClass (select (<= (Math|Random|RandomFloatinRange 0.0 1e+02) 35.0) "/Game/AdvanceAI/BP_AdvanceAI.BP_AdvanceAI_C" "/Game/Blueprints/TrackerBot/BP_TrackerBot.BP_TrackerBot_C") (Math|Transform|MakeTransform _array_element) "AdjustIfPossibleButDontSpawnIfColliding" 0 0)))))

(event EventBeginPlay
  (EventDispatchers|AssignOnActorKilled (delegate Custom|OnActorKilled_Event)))

(event EventTick
  (params (DeltaSeconds :type Float%20%28single-precision%29)))

(event EventSpawnNewBot
  (bind _returnvalue (AI|EQS|RunEQSQuery "/Game/AI/EQS_FindSpawnLocation.EQS_FindSpawnLocation" self "RandomBest25Pct")) ; Environment Query System (run asset EQS)
  (EventDispatchers|AssignOnQueryFinishedEvent _returnvalue (delegate Custom|OnQueryFinishedEvent_Event)))

(fn ConstructionScript)